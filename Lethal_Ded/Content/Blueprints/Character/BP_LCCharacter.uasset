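; BP_LCCharacter is a character Blueprint whose only active logic is a temporary developer speed control.
; When IA_Dev_SpeedControl starts, the sign of its axis value steps CurSpeed down or up by a fixed amount, staying strictly within minimum and maximum limits.
; While the action triggers, the current speed prints for debugging; this graph does not apply it to movement.
; BeginPlay, overlap, Tick and the construction script are empty.
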(event Input|EnhancedActionEvents|EnhancedInputActionIA_Dev_SpeedControl
  (params (ActionValue :type Float%20%28double-precision%29) (ElapsedSeconds :type Float%20%28double-precision%29) (TriggeredSeconds :type Float%20%28double-precision%29) (InputAction :type Input%20Action%20Object%20Reference :default "/Game/Blueprints/Character/Input/IA_Dev_SpeedControl.IA_Dev_SpeedControl"))
  ;[0.15 0.15 0.15 0.5] CharacterSpeedController(임시)
  (:Triggered
    (Development|PrintString (Utilities|String|ToString(Float) (Variables|Default|GetCurSpeed))))
  (:Started
    (Utilities|FlowControl|Sequence
      (:then_0
        (if (< ActionValue 0.0)
          (if (> (- (Variables|Default|GetCurSpeed) 2.0) 0.0)
            (Variables|Default|SetCurSpeed (- (Variables|Default|GetCurSpeed) 2.0)))))
      (:then_1
        (if (> ActionValue 0.0)
          (if (< (+ (Variables|Default|GetCurSpeed) 2.0) 2e+01)
            (Variables|Default|SetCurSpeed (+ (Variables|Default|GetCurSpeed) 2.0))))))))

(event EventBeginPlay)

(event Collision|EventActorBeginOverlap
  (params (OtherActor :type Actor%20Object%20Reference)))

(event EventTick
  (params (DeltaSeconds :type Float%20%28single-precision%29)))

(fn ConstructionScript)