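; Development player character Blueprint with temporary Enhanced Input handlers for moving, looking and tuning speed.
; Move input feeds AddMovementInput along actor forward and right vectors scaled by CurSpeed, which the dev speed action steps within fixed bounds and prints.
; Starting or stopping movement calls ChangeAnimationServer to switch upper and lower body montage sections between carry/walk and idle.
; Direct ABP_LCCharacterAnim walk and idle calls remain unconnected.
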(event Input|EnhancedActionEvents|EnhancedInputActionIA_Character_Move
  (params (ActionValue :type Vector%202D%20Structure) (ElapsedSeconds :type Float%20%28double-precision%29) (TriggeredSeconds :type Float%20%28double-precision%29) (InputAction :type Input%20Action%20Object%20Reference :default "/Game/Blueprints/Character/Input/IA_Character_Move.IA_Character_Move"))
  (bind _returnvalue (Transformation|GetActorForwardVector))
  (bind (_x _y) (Math|Vector2D|BreakVector2D ActionValue))
  (bind _returnvalue_2 (Transformation|GetActorRightVector))
  (bind _curspeed (Variables|Default|GetCurSpeed))
  (bind _curspeed_2 (Variables|Default|GetCurSpeed))
  ;[0.15 0.15 0.15 0.5] CharacterMove(임시)
  (:Triggered
    (Utilities|FlowControl|Sequence
      (:then_0
        (if (> _x 0.0)
          (Pawn|Input|AddMovementInput (* _returnvalue _curspeed_2) 0.2 false)))
      (:then_1
        (if (< _x 0.0)
          (Pawn|Input|AddMovementInput (* _returnvalue (* _curspeed_2 -1.0)) 0.2 false)))
      (:then_2
        (if (> _y 0.0)
          (Pawn|Input|AddMovementInput (* _returnvalue_2 _curspeed) 0.2 false)))
      (:then_3
        (if (< _y 0.0)
          (Pawn|Input|AddMovementInput (* _returnvalue_2 (* _curspeed -1.0)) 0.2 false)))))
  (:Started
    (Class|LCCharacter|ChangeAnimationServer "IDLE" "IDLE" "Carry_Upper" "Walk_Lower"))
  (:Completed
    (Class|LCCharacter|ChangeAnimationServer "IDLE" "IDLE" "Idle_Upper" "Idle_Lower")))

(event Input|EnhancedActionEvents|EnhancedInputActionIA_Dev_SpeedControl
  (params (ActionValue :type Float%20%28double-precision%29) (ElapsedSeconds :type Float%20%28double-precision%29) (TriggeredSeconds :type Float%20%28double-precision%29) (InputAction :type Input%20Action%20Object%20Reference :default "/Game/Blueprints/Character/Input/IA_Dev_SpeedControl.IA_Dev_SpeedControl"))
  ;[0.15 0.15 0.15 0.5] CharacterSpeedController(임시)
  (:Triggered
    (Development|PrintString (Utilities|String|ToString(Float) (Variables|Default|GetCurSpeed))))
  (:Started
    (Utilities|FlowControl|Sequence
      (:then_0
        (if (< ActionValue 0.0)
          (if (> (- (Variables|Default|GetCurSpeed) 2.0) 0.0)
            (Variables|Default|SetCurSpeed (- (Variables|Default|GetCurSpeed) 2.0)))))
      (:then_1
        (if (> ActionValue 0.0)
          (if (< (+ (Variables|Default|GetCurSpeed) 2.0) 2e+01)
            (Variables|Default|SetCurSpeed (+ (Variables|Default|GetCurSpeed) 2.0))))))))

(event Input|EnhancedActionEvents|EnhancedInputActionIA_Character_Rotate
  (params (ActionValue :type Vector%202D%20Structure) (ElapsedSeconds :type Float%20%28double-precision%29) (TriggeredSeconds :type Float%20%28double-precision%29) (InputAction :type Input%20Action%20Object%20Reference :default "/Game/Blueprints/Character/Input/IA_Character_Rotate.IA_Character_Rotate"))
  ;[0.15 0.15 0.15 0.5] CharacterRotate(임시)
  (Utilities|FlowControl|Sequence
    (:then_0
      (Pawn|Input|AddControllerYawInput (.x ActionValue)))
    (:then_1
      (Pawn|Input|AddControllerPitchInput (* (.y ActionValue) -1.0)))))

(event EventBeginPlay)

(event Collision|EventActorBeginOverlap
  (params (OtherActor :type Actor%20Object%20Reference)))

(event EventTick
  (params (DeltaSeconds :type Float%20%28single-precision%29)))

(fn ConstructionScript)