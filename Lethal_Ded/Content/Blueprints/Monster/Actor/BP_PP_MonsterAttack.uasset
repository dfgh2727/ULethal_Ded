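; BP_PP_MonsterAttack is an actor that switches on a post-process volume, named for monster attacks.
; C2S_PPEnable forwards to S2C_PPEnable, a relay named for client-to-server and server-to-client calls.
; S2C_PPEnable casts the PPV child actor to PostProcessVolume, enables it and prints its name, with no path to disable it.
; BeginPlay is empty, and a delayed local-controller trigger is left disconnected.
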(event Custom|C2S_PPEnable
  (CallFunction|S2CPPEnable))

(event Custom|S2C_PPEnable
  (bind _as포스트_프로세스_볼륨 (Utilities|Casting|CastToPostProcessVolume (Variables|/Script/Engine.ChildActorComponent|GetChildActor (Variables|Default|GetPPV))))
  (Variables|/Script/Engine.PostProcessVolume|SetbEnabled _as포스트_프로세스_볼륨 true)
  (Development|PrintString (Utilities|GetDisplayName _as포스트_프로세스_볼륨)))

(event EventBeginPlay)

(fn ConstructionScript)